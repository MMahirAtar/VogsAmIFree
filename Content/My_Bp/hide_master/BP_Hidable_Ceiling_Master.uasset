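; BP_Hidable_Ceiling_Master is a ceiling Blueprint that fades out and back in through its Hide and Show functions.
; BeginPlay creates a dynamic material from the mesh's first slot.
; While either flag is set, Tick calls UpdateVisibility to step the Opacity parameter by FaderSpeed times delta time, clearing the flag at the limit.
; An instanced-mesh row loop in the construction script is disconnected.
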(event `self.ReceiveTick`
  (params (DeltaSeconds :type "Float (single-precision)"))
  (bind _shouldhide (`self.ShouldHide`))
  (if _shouldhide
    (`self.UpdateVisibility` (* DeltaSeconds (`self.FaderSpeed`)) _shouldhide :!label _label)
    (elif (`self.ShouldShow`)
      (goto _label))))

(event `self.ReceiveBeginPlay`
  (bind _staticmesh (`self.StaticMesh`))
  (bind _returnvalue (`PrimitiveComponent.CreateDynamicMaterialInstance` _staticmesh 0 (`PrimitiveComponent.GetMaterial` _staticmesh 0)))
  (set `self.DynamicMaterial` _returnvalue))

(fn `Hide`
  (set `self.ShouldHide` true)
  (set `self.ShouldShow` false)
  (return))

(fn `Show`
  (set `self.ShouldShow` true)
  (set `self.ShouldHide` false)
  (return))

(fn `UpdateVisibility`
  (params (Amount :type "Float (double-precision)") (ShouldHide :type Boolean))
  (bind _dynamicmaterial (`self.DynamicMaterial`))
  (bind _returnvalue (`MaterialInstanceDynamic.K2_GetScalarParameterValue` _dynamicmaterial "Opacity"))
  (if ShouldHide
    (bind _returnvalue_2 (- _returnvalue Amount))
    (`MaterialInstanceDynamic.SetScalarParameterValue` _dynamicmaterial "Opacity" _returnvalue_2)
    (set `self.ShouldHide` (not (<= _returnvalue_2 0.0)))
    (else
      (bind _returnvalue_3 (+ _returnvalue Amount))
      (`MaterialInstanceDynamic.SetScalarParameterValue` _dynamicmaterial "Opacity" _returnvalue_3)
      (set `self.ShouldShow` (not (>= _returnvalue_3 1.0)))))
  (return))

(fn `UserConstructionScript`)